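; Game mode for a pinball game that runs the session from main menu through ball play to high score entry.
; Balls spawn at the plunger, and each one's destruction spawns the next until none remain, while AddScore applies the multiplier to points.
; Reset restores class defaults; game end opens high score entry if the saved list is short or beaten, otherwise the menu.
; High score save data is lazily loaded or created, then cached.
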(event Custom|SpawnBall
  (bind _returnvalue (Actor|GetActorOfClass "/Game/Blueprints/BP_Plunger.BP_Plunger_C"))
  (bind _returnvalue_2 (Game|SpawnActorfromClass "/Game/Blueprints/BP_Ball.BP_Ball_C" (Math|Transform|MakeTransform (Default|GetBallSpawnLocation _returnvalue) "0, 0, 0" "1,1,1") "Undefined" 0 0))
  (Game|BindEventtoOnDestroyed _returnvalue_2 (delegate Custom|OnBallDestroyed)))

(event Custom|OnBallDestroyed
  (params (DestroyedActor :type Actor%20Object%20Reference))
  (if (> (Variables|Default|GetBallsRemaining) 0)
    (CallFunction|SpawnBall)
    (Math|Integer|DecrementInt (Variables|Default|GetBallsRemaining))
    (else
      (CallFunction|Endgame))))

(event Custom|Endgame
  (bind _currentsaveobject (CallFunction|GetSaveGameData))
  (if (<= (Utilities|Array|Length (Variables|/Game/Blueprints/BP_HighscoreSave.BP_HighscoreSave_C|GetSaveStruct _currentsaveobject)) 3)
    (CallFunction|CreateHighScoreList :!label _label)
    (else
      (bind _lowestscorestruct (Default|GetLowestScore _currentsaveobject))
      (if (< (.score _lowestscorestruct) (Variables|Default|GetScore))
        (goto _label)
        (else
          (CallFunction|CreateMainMenu))))))

(event Custom|CreateHighScoreList
  (bind _returnvalue (Game|GetPlayerController 0))
  (bind _asbp_pinball_player_controller (Utilities|Casting|CastToBP_PinballPlayerController _returnvalue))
  (bind _returnvalue_2 (UserInterface|CreateWidget "/Game/Blueprints/UMG_HighScoreEntry.UMG_HighScoreEntry_C" _asbp_pinball_player_controller))
  (UserInterface|Viewport|AddtoViewport _returnvalue_2 0)
  (Variables|/Script/Engine.PlayerController|SetbShowMouseCursor _asbp_pinball_player_controller true))

(event Custom|CreateMainMenu
  (bind _returnvalue (Game|GetPlayerController 0))
  (bind _asbp_pinball_player_controller (Utilities|Casting|CastToBP_PinballPlayerController _returnvalue))
  (CallFunction|GetSaveGameData)
  (Viewport|RemoveAllWidgets)
  (bind _returnvalue_2 (UserInterface|CreateWidget "/Game/Blueprints/UMG_MainMenu.UMG_MainMenu_C" _asbp_pinball_player_controller))
  (UserInterface|Viewport|AddtoViewport _returnvalue_2 0)
  (Variables|/Script/Engine.PlayerController|SetbShowMouseCursor _asbp_pinball_player_controller true))

(event Custom|ResetGame
  (bind _returnvalue (Game|GetPlayerController 0))
  (bind (_multiplier _score _ballsremaining _currentsaveobject _highscoresavename _ongamereset _tiltcount) (Utilities|GetClassDefaults "BP_Gamemode_C"))
  (bind _asbp_pinball_player_controller (Utilities|Casting|CastToBP_PinballPlayerController _returnvalue))
  (Variables|Default|SetTiltCount _tiltcount)
  (Variables|Default|SetScore _score)
  (Variables|Default|SetMultiplier _multiplier)
  (Variables|Default|SetBallsRemaining _ballsremaining)
  (CallFunction|SpawnBall)
  (Default|CreatePlayerHUD _asbp_pinball_player_controller)
  (Variables|/Script/Engine.PlayerController|SetbShowMouseCursor _asbp_pinball_player_controller false)
  (Default|CallOnGameReset))

(event EventBeginPlay
  (CallFunction|CreateMainMenu)
  (Audio|PlaySound2D "/Game/Assets/Sounds/victoryMusic_loop_01.victoryMusic_loop_01" 0.1 1.0 0.0 0 0))

(event EventTick
  (params (DeltaSeconds :type Float%20%28single-precision%29)))

(fn ConstructionScript)

(fn AddScore
  (params (PointsToAdd :type Float%20%28single-precision%29))
  (bind _output_get (Variables|Default|SetScore (+ (* PointsToAdd (Variables|Default|GetMultiplier)) (Variables|Default|GetScore))))
  (return _output_get))

(fn GetSaveGameData
  (bind _currentsaveobject (Variables|Default|GetCurrentSaveObject)
    (:then
      (return _currentsaveobject))
    (:else
      (bind _returnvalue (SaveGame|DoesSaveGameExist (Variables|Default|GetHighScoreSaveName)))
      (if _returnvalue
        (bind _returnvalue_2 (SaveGame|LoadGamefromSlot (Variables|Default|GetHighScoreSaveName)))
        (bind _asbp_highscore_save (Utilities|Casting|CastToBP_HighscoreSave _returnvalue_2)
          (:then
            (Default|SortSaveData _asbp_highscore_save)
            (bind _output_get (Variables|Default|SetCurrentSaveObject _asbp_highscore_save))
            (return _output_get))
          (:CastFailed
            _))
        (else
          (bind _returnvalue_3 (SaveGame|CreateSaveGameObject "/Game/Blueprints/BP_HighscoreSave.BP_HighscoreSave_C"))
          (bind _asbp_highscore_save_2 (Utilities|Casting|CastToBP_HighscoreSave _returnvalue_3)
            (:then
              (bind _output_get_2 (Variables|Default|SetCurrentSaveObject _asbp_highscore_save_2))
              (return _output_get_2))
            (:CastFailed
              _))))
      (return 0))))