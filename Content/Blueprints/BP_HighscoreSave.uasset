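; BP_HighscoreSave holds the high score list and keeps it ranked from highest to lowest, capped at four entries.
; AddHighScore appends the new entry, calls SortSaveData, then trims the array.
; SortSaveData is a selection sort that repeatedly moves the GetHighestScore result into a temporary array, then copies it back.
; GetLowestScore returns the weakest entry and its index but is not called within this Blueprint.
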(fn GetLowestScore
  (bind _savestruct (Variables|Default|GetSaveStruct))
  (for (_array_element _array_index) _savestruct
    (if (== _array_index 0)
      (LocalVariables|SetLowestScore (.score _array_element))
      (LocalVariables|SetLowestIndex _array_index)
      (elif (< (.score _array_element) (LocalVariables|GetLowestScore))
        (LocalVariables|SetLowestScore (.score _array_element))
        (LocalVariables|SetLowestIndex _array_index))))
  (return (Utilities|Array|Get(acopy) _savestruct (LocalVariables|GetLowestIndex)) (LocalVariables|GetLowestIndex)))

(fn GetHighestScore
  (bind _savestruct (Variables|Default|GetSaveStruct))
  (for (_array_element _array_index) _savestruct
    (if (== _array_index 0)
      (LocalVariables|SetHighestScore (.score _array_element))
      (LocalVariables|SetHighestIndex _array_index)
      (elif (> (.score _array_element) (LocalVariables|GetHighestScore))
        (LocalVariables|SetHighestScore (.score _array_element))
        (LocalVariables|SetHighestIndex _array_index))))
  (return (Utilities|Array|Get(acopy) _savestruct (LocalVariables|GetHighestIndex)) (LocalVariables|GetHighestIndex)))

(fn SortSaveData
  (while (> (Utilities|Array|Length (Variables|Default|GetSaveStruct)) 0)
    (bind (_highestscorestruct _highestscoreindex) (CallFunction|GetHighestScore))
    (Utilities|Array|Add (LocalVariables|GetTempSaveStruct) _highestscorestruct)
    (Utilities|Array|RemoveIndex (Variables|Default|GetSaveStruct) _highestscoreindex))
  (Variables|Default|SetSaveStruct (LocalVariables|GetTempSaveStruct)))

(fn AddHighScore
  (params (NewScore :type High%20Score%20Struct%20Structure))
  (bind _savestruct (Variables|Default|GetSaveStruct))
  (Utilities|Array|Add (Variables|Default|GetSaveStruct) NewScore)
  (CallFunction|SortSaveData)
  (Utilities|Array|Resize _savestruct (Math|Integer|Min(Integer) (Utilities|Array|Length _savestruct) 4)))