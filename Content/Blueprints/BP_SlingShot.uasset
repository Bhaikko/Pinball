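; BP_SlingShot is a pinball-style slingshot bumper that kicks the ball away on contact.
; On overlap with a BP_Ball it adds score through BP_Gamemode and applies an impulse to the ball opposite the mesh's forward vector.
; A SlingBounce timeline then animates the PercentOut parameter on a dynamic material instance, created for mesh slot 2 in the construction script, as bounce feedback.
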(event EventBeginPlay)

(event Collision|EventActorBeginOverlap
  (params (OtherActor :type Actor%20Object%20Reference))
  (bind _asbp_ball (Utilities|Casting|CastToBP_Ball OtherActor))
  (bind _asbp_gamemode (Utilities|Casting|CastToBP_Gamemode (Game|GetGameMode)))
  (Default|AddScore _asbp_gamemode 2e+01)
  (Physics|AddImpulse (Variables|/Game/Blueprints/BP_Ball.BP_Ball_C|GetBall _asbp_ball) (* (Math|Vector|GetForwardVector (Variables|Default|GetStaticMesh)) -2.5e+03) "None" false)
  (bind _newtrack_0 (Timeline|SlingBounce PlayFromStart)
    (:Update
      (bind _asmaterial_instance_dynamic (Utilities|Casting|CastToMaterialInstanceDynamic (Rendering|Material|GetMaterial (Variables|Default|GetStaticMesh) 2)))
      (Rendering|Material|SetScalarParameterValue _asmaterial_instance_dynamic "PercentOut" _newtrack_0 :!class /Script/Engine.MaterialInstanceDynamic))))

(event EventTick
  (params (DeltaSeconds :type Float%20%28single-precision%29)))

(fn ConstructionScript
  ;[1 1 1] Creating Material Instance Programatically
  (Rendering|Material|CreateDynamicMaterialInstance (Variables|Default|GetStaticMesh) 2 0 "None" :!class /Script/Engine.PrimitiveComponent))